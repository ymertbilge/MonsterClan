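; BPC_Currencies is a currency component that holds the player's Gold balance.
; Events add five times a transferred item's value, deduct spent gold without a balance check, or grant a fixed cheat bonus.
; After each change it sends the new total to player controller 0 through a currency-to-UI update message.
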(event `self.ReceiveBeginPlay`)

(event `TransferItemValue`
  (params (ItemValue :type Integer))
  (bind _output_get (set `self.Gold` (+ (* ItemValue 5) (`self.Gold`))))
  (message `/Game/GameSystems/Interfaces/BPI_UIActions.UpdateCurrencyToUI` (`GameplayStatics.GetPlayerController` 0) _output_get))

(event `Spend Gold`
  (params (`Gold to Deduce` :type Integer))
  (bind _output_get (set `self.Gold` (- (`self.Gold`) `Gold to Deduce`)))
  (message `/Game/GameSystems/Interfaces/BPI_UIActions.UpdateCurrencyToUI` (`GameplayStatics.GetPlayerController` 0) _output_get))

(event `GainGold (Cheat)`
  (bind _output_get (set `self.Gold` (+ 100 (`self.Gold`))))
  (message `/Game/GameSystems/Interfaces/BPI_UIActions.UpdateCurrencyToUI` (`GameplayStatics.GetPlayerController` 0) _output_get))