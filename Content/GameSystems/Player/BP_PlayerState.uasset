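; Player state Blueprint that fronts the player's resources and currencies through BPCResources and BPCCurrencies components.
; Adding or selling resources updates the resource map and messages the first player controller to refresh the UI.
; A sale requires and removes five units, then passes the resource's base value to the currency component, which also handles gold spending.
; Fetch functions expose currency totals and storage, while the other getters are empty stubs.
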(event `/Game/GameSystems/Resources/BPI_Resource.Add Resource`
  (params (`Resource Type` :type "/Game/GameSystems/Resources/PDA_Resources Object Reference") (Amount :type Integer))
  (bind _resources (`/Game/GameSystems/Resources/BPC_Resources.Resources` (`self.BPC_Resources`)))
  (`BlueprintMapLibrary.Map_Add` _resources `Resource Type` (+ (`BlueprintMapLibrary.Map_Find` _resources `Resource Type`) Amount))
  (message `/Game/GameSystems/Interfaces/BPI_UIActions.UpdateResourcesToUI` (`GameplayStatics.GetPlayerController` 0)))

(event `/Game/GameSystems/Interfaces/BPI_UIActions.SellResource (Test)`
  (params (Resource :type "/Game/GameSystems/Resources/PDA_Resources Object Reference"))
  (bind _bpc_resources (`self.BPC_Resources`))
  (bind _value (`BlueprintMapLibrary.Map_Find` (`/Game/GameSystems/Resources/BPC_Resources.Resources` _bpc_resources) Resource))
  (if (>= _value 5)
    (`BlueprintMapLibrary.Map_Add` (`/Game/GameSystems/Resources/BPC_Resources.Resources` _bpc_resources) Resource (- _value 5))
    (message `/Game/GameSystems/Interfaces/BPI_UIActions.UpdateResourcesToUI` (`GameplayStatics.GetPlayerController` 0))
    (`/Game/GameSystems/Currencies/BPC_Currencies.TransferItemValue` (`self.BPC_Currencies`) (`/Game/GameSystems/Resources/PDA_Resources.BaseValue` Resource))))

(event `/Game/GameSystems/Interfaces/BPI_UIActions.SpendGold`
  (params (`Gold Amount` :type Integer))
  (`/Game/GameSystems/Currencies/BPC_Currencies.Spend Gold` (`self.BPC_Currencies`) `Gold Amount`))

(fn `FetchCurrencyData`
  (returns (`Gold Amount` :type Integer) (`Sigil Amount` :type Integer) (`Reputation Amount` :type Integer))
  (bind _bpc_currencies (`self.BPC_Currencies`))
  (return (`/Game/GameSystems/Currencies/BPC_Currencies.Gold` _bpc_currencies) (`/Game/GameSystems/Currencies/BPC_Currencies.ElderSigils` _bpc_currencies) (`/Game/GameSystems/Currencies/BPC_Currencies.GuildReputation` _bpc_currencies)))

(fn `FetchStorageData`
  (returns (Resources :type "Map of /Game/GameSystems/Resources/PDA_Resources Object Reference to Integer"))
  (return (`/Game/GameSystems/Resources/BPC_Resources.Resources` (`self.BPC_Resources`))))

(fn `Get Current Resources`
  (returns (Resources :type "Map of /Game/GameSystems/Resources/PDA_Resources Object Reference to Integer"))
  (return))

(fn `Get HUD`
  (returns (HUD :type "/Game/GameSystems/UserInterface/WBP_MainHUD Object Reference"))
  (return null))

(fn `Get Room Upgrade Tree`
  (returns (`Upgrade Tree` :type "UserWidget Object Reference"))
  (return null))

(fn `GetActiveUI`
  (returns (`Active UI` :type "Widget Object Reference"))
  (return null))

(fn `UserConstructionScript`)