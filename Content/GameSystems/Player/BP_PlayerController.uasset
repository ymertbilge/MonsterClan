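; Player controller that sets up general input and the main HUD, and gives access to the player's resource amounts.
; On BeginPlay it caches the BP_PlayerState, then, if the Enhanced Input subsystem is valid, adds the general mapping context and creates the HUD.
; It passes itself to the gold, reputation and sigil widgets as their player actor.
; GetResourceAmount looks up a named resource's current amount in the player state's resources component.
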(event `self.ReceiveBeginPlay`
  (bind _returnvalue (subsystem `EnhancedInputLocalPlayerSubsystem`))
  (bind _asbp_player_state (cast `/Game/GameSystems/Player/BP_PlayerState` (`GameplayStatics.GetPlayerState` 0)))
  (set `self.PlayerStateRef` _asbp_player_state)
  (`/Engine/EditorBlueprintResources/StandardMacros.IsValid` _returnvalue
    (:`Is Valid`
      (`EnhancedInputSubsystemInterface.AddMappingContext` _returnvalue "/Game/Input/IMC_General.IMC_General" 0 (struct))
      (bind _returnvalue_2 (`|CreateWidget` "/Game/GameSystems/UserInterface/WBP_MainHUD.WBP_MainHUD_C"))
      (`UserWidget.AddToViewport` _returnvalue_2 0)
      (bind _wbp_resourcebar (`/Game/GameSystems/UserInterface/WBP_MainHUD.WBP_ResourceBar` _returnvalue_2))
      (set `/Game/GameSystems/UserInterface/WBP_Resource.PlayerActor` self (`/Game/GameSystems/UserInterface/WBP_ResourceBar.WBP_Resource_Gold` _wbp_resourcebar))
      (set `/Game/GameSystems/UserInterface/WBP_Resource.PlayerActor` self (`/Game/GameSystems/UserInterface/WBP_ResourceBar.WBP_Resource_Reputation` _wbp_resourcebar))
      (set `/Game/GameSystems/UserInterface/WBP_Resource.PlayerActor` self (`/Game/GameSystems/UserInterface/WBP_ResourceBar.WBP_Resource_Sigil` _wbp_resourcebar)))))

(fn `GetResourceAmount`
  (params (`Resource Name` :type "/Game/GameSystems/Resources/E_ResourceType Enum" :default "NewEnumerator3"))
  (returns (Amount :type "Float (double-precision)"))
  (return (`.CurrentAmount_24_79D4420E452B2E76E1C186955B86B467` (break `/Game/GameSystems/Resources/FResourceData` (`BlueprintMapLibrary.Map_Find` (`/Game/GameSystems/Resources/BPC_Resources.Resources` (`/Game/GameSystems/Player/BP_PlayerState.BPC_Resources` (`self.PlayerStateRef`))) `Resource Name`)))))

(fn `UserConstructionScript`)