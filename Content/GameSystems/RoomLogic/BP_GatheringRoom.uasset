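; BP_GatheringRoom is a room where the player spends gold on a timed contract to gather resources, configured from DT_GatheringRooms.
; An active contract runs timers for gathering, duration and progress bar updates; cancelling clears gathering and progress timers.
; Each gather rolls against equipment skill for primary and possible secondary resources, or one primary on failure, crediting PlayerState and showing popups.
; Unit lookup and storage fetch are empty stubs.
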(event `/Game/GameSystems/Interfaces/BPI_Interaction.Interact`
  (`parent.Interact`)
  (message `/Game/GameSystems/Interfaces/BPI_UIActions.TransferGatheringRoomData` (`self.RoomUI`) (`self.GatheringRoomData`)))

(event `ResetContract`
  (`KismetSystemLibrary.K2_ClearAndInvalidateTimerHandle` (`self.GatheringOperationHandle`) :!label _label)
  (`KismetSystemLibrary.K2_ClearAndInvalidateTimerHandle` (`self.ContractProgressTimer`))
  (`TextBlock.SetText` (`/Game/GameSystems/UserInterface/WBP_GatheringRoomBase.TB_ButtonText` (`self.RoomUI`)) "Buy Contract")
  (set `self.ContractActive` false)
  (`/Game/GameSystems/UserInterface/WBP_GatheringRoomBase.TransferContractStatus` (`self.RoomUI`) false)
  (`Widget.SetVisibility` (`/Game/GameSystems/UserInterface/WBP_GatheringRoomBase.WBP_ContractTimer` (`self.RoomUI`)) "Collapsed"))

(event `/Game/GameSystems/Interfaces/BPI_UIActions.CheckContract`
  (params (`Contract Price` :type Integer))
  (bind ((`ContractPrice_71_BC18A8F649E9511BEAD72CAB1A636960` _contractprice) (`ContractTime_78_77996D47488A64D2BDA34B88804561E4` _contracttime)) (break `/Game/GameSystems/RoomLogic/FGatheringRoomStruct` (`self.GatheringRoomData`)))
  (if (not (`self.ContractActive`))
    (bind _gold_amount (message `/Game/GameSystems/Interfaces/BPI_UIActions.FetchCurrencyData` (`GameplayStatics.GetPlayerState` 0)))
    (if (>= _gold_amount `Contract Price`)
      (set `self.ContractActive` true)
      (bind _returnvalue (`KismetSystemLibrary.K2_SetTimerDelegate` (`|CreateDelegate` :!event `GatheringOperation`) 2.0 true))
      (set `self.GatheringOperationHandle` _returnvalue)
      (`TextBlock.SetText` (`/Game/GameSystems/UserInterface/WBP_GatheringRoomBase.TB_ButtonText` (`self.RoomUI`)) "Cancel Contract")
      (`/Game/GameSystems/UserInterface/WBP_GatheringRoomBase.TransferContractStatus` (`self.RoomUI`) true)
      (message `/Game/GameSystems/Interfaces/BPI_UIActions.SpendGold` (`GameplayStatics.GetPlayerState` 0) _contractprice)
      (bind _returnvalue_2 (`KismetSystemLibrary.K2_SetTimerDelegate` (`|CreateDelegate` :!event `ResetContract`) _contracttime))
      (set `self.ContractTimerHandle` _returnvalue_2)
      (`Widget.SetVisibility` (`/Game/GameSystems/UserInterface/WBP_GatheringRoomBase.WBP_ContractTimer` (`self.RoomUI`)) "Visible")
      (bind _returnvalue_3 (`KismetSystemLibrary.K2_SetTimerDelegate` (`|CreateDelegate` :!event `UpdateContractProgressUI`) 0.1 true))
      (set `self.ContractProgressTimer` _returnvalue_3))
    (else
      (goto _label))))

(event `UpdateContractProgressUI`
  (bind (_percent _remaining_seconds) (`self.GetContractTimeData`))
  (bind _wbp_contracttimer (`/Game/GameSystems/UserInterface/WBP_GatheringRoomBase.WBP_ContractTimer` (`self.RoomUI`)))
  (`/Game/GameSystems/UserInterface/WBP_ContractTimer.UpdateTimerBar` _wbp_contracttimer _percent)
  (`/Game/GameSystems/UserInterface/WBP_ContractTimer.UpdateTimerText` _wbp_contracttimer _remaining_seconds))

(event `GatheringOperation`
  (`self.TryGatherResource`))

(fn `FetchStorageData`
  (returns (Resources :type "Map of /Game/GameSystems/Resources/PDA_Resources Object Reference to Integer"))
  (return))

(fn `GatherResource`
  (params (`Resource Type` :type "/Game/GameSystems/Resources/PDA_Resources Object Reference") (Amount :type Integer))
  (message `/Game/GameSystems/Resources/BPI_Resource.Add Resource` (`GameplayStatics.GetPlayerState` 0) `Resource Type` Amount)
  (`self.OnResourceGathered`)
  (return))

(fn `GetAssignedUnit`
  (returns (AssignedUnit :type "Actor Object Reference"))
  (return null))

(fn `GetContractTimeData`
  (returns (Percent :type "Float (double-precision)") (`Remaining Seconds` :type "Float (double-precision)"))
  (bind ((`ContractTime_78_77996D47488A64D2BDA34B88804561E4` _contracttime)) (break `/Game/GameSystems/RoomLogic/FGatheringRoomStruct` (`self.GatheringRoomData`)))
  (bind _returnvalue (`KismetSystemLibrary.K2_GetTimerRemainingTimeHandle` (`self.ContractTimerHandle`)))
  (return (`KismetMathLibrary.NormalizeToRange` (`KismetMathLibrary.FClamp` _returnvalue 0.0 _contracttime) 0.0 _contracttime) _returnvalue))

(fn `InitializeRoomData`
  (bind _returnvalue (`|GetDataTableRow` "/Game/GameSystems/RoomLogic/DT_GatheringRooms.DT_GatheringRooms" (`self.Name`))
    (:`then`
      (set `self.GatheringRoomData` _returnvalue))))

(fn `TryGatherResource`
  (returns (`Return value` :type Boolean))
  (bind _primaryresource (`self.PrimaryResource`))
  (bind _primaryresource_2 (`self.PrimaryResource`))
  (bind _secondaryresource (`self.SecondaryResource`))
  (bind _primaryresource_3 (`self.PrimaryResource`))
  (bind _primaryresource_4 (`self.PrimaryResource`))
  (bind ((`ProducedResources_62_6EF2B70E4D9B893EE866389B5E48F08B` _producedresources)) (break `/Game/GameSystems/RoomLogic/FGatheringRoomStruct` (`self.GatheringRoomData`)))
  (bind ((`ProducedResources_62_6EF2B70E4D9B893EE866389B5E48F08B` _producedresources_2)) (break `/Game/GameSystems/RoomLogic/FGatheringRoomStruct` (`self.GatheringRoomData`)))
  (if (<= (`KismetMathLibrary.RandomIntegerInRange` 1 100) (+ (`.BaseEquipmentSkill_70_70307D654FC93845FC6BB5BFF7718BA4` (break `/Game/GameSystems/RoomLogic/FGatheringRoomStruct` (`self.GatheringRoomData`))) 0))
    (if (< (`KismetMathLibrary.RandomFloatInRange` 0.0 1.0) 0.75)
      (`self.GatherResource` _primaryresource_4 (`BlueprintMapLibrary.Map_Find` _producedresources _primaryresource_4))
      (else
        (`self.GatherResource` _secondaryresource (`BlueprintMapLibrary.Map_Find` _producedresources _secondaryresource))
        (`self.GatherResource` _primaryresource_2 (`BlueprintMapLibrary.Map_Find` _producedresources _primaryresource_2))
        (message `/Game/GameSystems/Interfaces/BPI_UIActions.UpdatePopupUI` (`WidgetComponent.GetWidget` (`self.WC_Secondary_PopUp`)) (`/Game/GameSystems/Resources/PDA_Resources.Icon` (`self.SecondaryResource`)) (`BlueprintMapLibrary.Map_Find` (`.ProducedResources_62_6EF2B70E4D9B893EE866389B5E48F08B` (break `/Game/GameSystems/RoomLogic/FGatheringRoomStruct` (`self.GatheringRoomData`))) (`self.SecondaryResource`)))))
    (if (<= (`KismetMathLibrary.RandomIntegerInRange` 1 100) (/ 0 2))
      (`self.GatherResource` _primaryresource (`BlueprintMapLibrary.Map_Find` _producedresources_2 _primaryresource))
      (message `/Game/GameSystems/Interfaces/BPI_UIActions.UpdatePopupUI` (`WidgetComponent.GetWidget` (`self.WC_Main_PopUp`)) (`/Game/GameSystems/Resources/PDA_Resources.Icon` (`self.PrimaryResource`)) (* (`BlueprintMapLibrary.Map_Find` _producedresources_2 (`self.PrimaryResource`)) 2))
      (return true)
      (else
        (message `/Game/GameSystems/Interfaces/BPI_UIActions.UpdatePopupUI` (`WidgetComponent.GetWidget` (`self.WC_Main_PopUp`)) (`/Game/GameSystems/Resources/PDA_Resources.Icon` (`self.PrimaryResource`)) (`BlueprintMapLibrary.Map_Find` (`.ProducedResources_62_6EF2B70E4D9B893EE866389B5E48F08B` (break `/Game/GameSystems/RoomLogic/FGatheringRoomStruct` (`self.GatheringRoomData`))) (`self.PrimaryResource`)))
        (return true)))
    (else
      (`self.GatherResource` _primaryresource_3 1)
      (message `/Game/GameSystems/Interfaces/BPI_UIActions.UpdatePopupUI` (`WidgetComponent.GetWidget` (`self.WC_Main_PopUp`)) (`/Game/GameSystems/Resources/PDA_Resources.Icon` _primaryresource_3) 1)
      (return false))))

(fn `UserConstructionScript`
  (`parent.UserConstructionScript`)
  (`self.InitializeRoomData`))