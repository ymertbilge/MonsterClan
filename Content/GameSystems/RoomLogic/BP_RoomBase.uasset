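; BP_RoomBase is a base room actor that toggles a highlight and room UI on selection changes, passing Interact to its parent.
; Highlighting swaps an overlay material on the mesh.
; ToggleRoomUI creates or removes a RoomType-specific widget (only Gathering builds one) in the HUD's RoomBox, tracking the active one on the player controller.
; Currency, storage, HUD and other UI getters are empty stubs or return defaults.
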(event `/Game/GameSystems/Interfaces/BPI_Interaction.Interact`
  (`parent.Interact`))

(event `/Game/GameSystems/Interfaces/BPI_Interaction.ClearPreviousSelection`
  (`self.SetHighlight`)
  (`self.ToggleRoomUI`))

(fn `CreateRoomWidget`
  (returns (`Return Widget` :type "/Game/GameSystems/UserInterface/WBP_GatheringRoomBase Object Reference"))
  (switch `/Game/GameSystems/RoomLogic/E_RoomTypes` (`self.RoomType`)
    (:`NewEnumerator4`
      (`self.DestroyRoomWidget`))
    (:`NewEnumerator1`
      (bind _hud (message `/Game/GameSystems/Interfaces/BPI_UIActions.Get HUD` (`GameplayStatics.GetPlayerController` 0)))
      (`PanelWidget.ClearChildren` (`/Game/GameSystems/UserInterface/WBP_MainHUD.RoomBox` _hud))
      (bind _returnvalue (`|CreateWidget` "/Game/GameSystems/UserInterface/WBP_GatheringRoomBase.WBP_GatheringRoomBase_C"))
      (`PanelWidget.AddChild` (`/Game/GameSystems/UserInterface/WBP_MainHUD.RoomBox` _hud) _returnvalue)
      (`Widget.SetVisibility` _returnvalue "Visible")
      (return _returnvalue))))

(fn `DestroyRoomWidget`
  (bind _roomui (`self.RoomUI`))
  (`Widget.RemoveFromParent` _roomui)
  (`Widget.SetVisibility` _roomui "Collapsed")
  (return))

(fn `FetchCurrencyData`
  (returns (`Gold Amount` :type Integer) (`Sigil Amount` :type Integer) (`Reputation Amount` :type Integer))
  (return 0 0 0))

(fn `FetchStorageData`
  (returns (Resources :type "Map of /Game/GameSystems/Resources/PDA_Resources Object Reference to Integer"))
  (return))

(fn `Get HUD`)

(fn `Get Upgrade Details Widget`
  (returns (Upgrade :type "UserWidget Object Reference"))
  (return null))

(fn `GetActiveUI`
  (returns (`Active UI` :type "Widget Object Reference"))
  (return null))

(fn `SetHighlight`
  (bind _mesh (`self.Mesh`))
  (if (not (`self.IsHighlighted`))
    (`MeshComponent.SetOverlayMaterial` _mesh "/Game/GameSystems/Materials/M_Highlight.M_Highlight")
    (set `self.IsHighlighted` true)
    (else
      (`MeshComponent.SetOverlayMaterial` _mesh null)
      (set `self.IsHighlighted` false))))

(fn `ToggleRoomUI`
  (returns (`Active Widget` :type "Widget Object Reference"))
  (bind _returnvalue (`GameplayStatics.GetPlayerController` 0))
  (bind _active_ui (message `/Game/GameSystems/Interfaces/BPI_UIActions.GetActiveUI` (`GameplayStatics.GetPlayerController` 0)))
  (`/Engine/EditorBlueprintResources/StandardMacros.IsValid` _active_ui
    (:`Is Valid`
      (if (== (`self.RoomUI`) _active_ui)
        (`self.DestroyRoomWidget`)
        (set `self.RoomUI` null)
        (message `/Game/GameSystems/Interfaces/BPI_UIActions.SetActiveUI` _returnvalue null)
        (else
          (bind _return_widget (`self.CreateRoomWidget` :!label _label))
          (bind _output_get (set `self.RoomUI` _return_widget))
          (message `/Game/GameSystems/Interfaces/BPI_UIActions.SetActiveUI` _returnvalue _output_get))))
    (:`Is Not Valid`
      (goto _label)))
  (return (`self.RoomUI`)))

(fn `UserConstructionScript`)